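; Player-controlled physics blob that moves by impulses and switches between a soft state and a hard state.
; Tick applies axis-input impulses, counters speed above a limit and adds extra downward gravity.
; Holding SwitchState changes power, speed limit, gravity, mass and materials; releasing restores them with a full-soft physical material until a tick countdown switches it to half-soft.
; R resets position and velocity; an upward impulse branch is unconnected.
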(event `self.ReceiveBeginPlay`
  ;[1 1 1] Set Startup Values (Makes it so you don't have to set two variables when modifying them)
  (set `self.CurPower` (`self.BasePower`))
  (set `self.CurVelLim` (`self.BaseVelLim`))
  (set `self.CurGrav` (`self.BaseGrav`)))

(event `Key|R`
  (params (Key :type "Key Structure"))
  (bind _char (`self.Char`))
  ;[1 1 1] Reset
  (:`Pressed`
    (`SceneComponent.K2_SetWorldLocation` _char (0.0 0.0 1000.0) false false)
    (`PrimitiveComponent.SetPhysicsLinearVelocity` _char (0.0 0.0 0.0) false "None")))

(event `self.ReceiveTick`
  (params (DeltaSeconds :type "Float (single-precision)"))
  (bind _char (`self.Char`))
  (bind _curpower (`self.CurPower`))
  ;[1 1 1] Add Movement Velocity
  (`PrimitiveComponent.AddImpulse` _char (* (`KismetMathLibrary.Normal` (`KismetMathLibrary.MakeVector` (`self.GetInputAxisValue`) (`self.GetInputAxisValue`))) _curpower) "None" false)
  ;[1 1 1] Limit Velocity
  (bind _returnvalue (`PrimitiveComponent.GetPhysicsLinearVelocity` _char "None"))
  (if (> (`KismetMathLibrary.VSize` _returnvalue) (`self.CurVelLim`))
    (`PrimitiveComponent.AddImpulse` _char (* (* (`KismetMathLibrary.Normal` _returnvalue) -1) _curpower) "None" false))
  ;[1 1 1] Add Extra Gravity
  (`PrimitiveComponent.AddImpulse` _char (* (0.0 0.0 -1.0) (`self.CurGrav`)) "None" false)
  ;[1 1 1] Countdown Bounce Frame Timer
  (if (== 0 (`self.BounceTimer`))
    (`PrimitiveComponent.SetPhysMaterialOverride` _char "/Game/phys_mat/SoftHalf_PM.SoftHalf_PM"))
  (`/Engine/EditorBlueprintResources/StandardMacros.DecrementInt` (`self.BounceTimer`)))

(event `InputAction|Jump`
  (params (Key :type "Key Structure"))
  ;[1 1 1] Jump while in soft state
)

(event `InputAction|SwitchState`
  (params (Key :type "Key Structure"))
  (bind _hardmovemultiplier (`self.HardMoveMultiplier`))
  (bind _mass (`self.Mass`))
  (bind _basegrav (`self.BaseGrav`))
  (bind _basepower (`self.BasePower`))
  (bind _basevellim (`self.BaseVelLim`))
  (bind _char (`self.Char`))
  ;[1 1 1] Switch state
  (:`Pressed`
    (set `self.State` 1)
    (set `self.CurPower` (* _basepower _hardmovemultiplier))
    (set `self.CurVelLim` (* _basevellim _hardmovemultiplier))
    (set `self.CurGrav` (* _basegrav (`self.HardGravModifier`)))
    (`PrimitiveComponent.SetMassOverrideInKg` _char "None" (* _mass _hardmovemultiplier) true)
    (`PrimitiveComponent.SetMaterial` _char 0 "/Engine/MapTemplates/Sky/Desert_Outer_HDR_Mat.Desert_Outer_HDR_Mat")
    (`PrimitiveComponent.SetPhysMaterialOverride` _char "/Game/phys_mat/Hard_PM.Hard_PM"))
  (:`Released`
    (set `self.State` 0)
    (set `self.CurPower` _basepower)
    (set `self.CurVelLim` _basevellim)
    (set `self.CurGrav` _basegrav)
    (`PrimitiveComponent.SetMassOverrideInKg` _char "None" _mass true)
    (`PrimitiveComponent.SetMaterial` _char 0 "/Engine/EngineMaterials/DefaultMaterial.DefaultMaterial")
    (`PrimitiveComponent.SetPhysMaterialOverride` _char "/Game/phys_mat/SoftFull_PM.SoftFull_PM")
    (set `self.BounceTimer` (`self.BounceTimerSet`))))

(fn `UserConstructionScript`)