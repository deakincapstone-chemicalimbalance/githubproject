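; Physics-driven blob player prototype that rolls on impulses and switches between soft, held-hard and float-powerup states, changing mass, physical material and movement tuning.
; Tick sphere-traces for ground, applies input, speed limiting and extra gravity, and runs jump and bounce timers, the latter briefly boosting bounce material after softening.
; Hard and soft morph AnimInstances fake rolling from velocity, state transitions and landing squish.
; Overlaps grant float or one-shot speed boosts; audio follows movement, jumps and landings.
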(event `self.ReceiveBeginPlay`
  ;[1 1 1] Set Startup Values
  (set `self.CurPower` (`self.BasePower`))
  (set `self.CurVelLim` (`self.BaseVelLim`))
  (set `self.CurGrav` (`self.BaseGrav`))
  (bind _ashard_state_anim (cast `/Game/Models/Blob/HardStateAnim` (`SkeletalMeshComponent.GetAnimInstance` (`self.HardStateMorph`))))
  (set `self.HardStateAnim` _ashard_state_anim)
  (bind _assoft_state_anim (cast `/Game/Models/Blob/SoftStateAnim` (`SkeletalMeshComponent.GetAnimInstance` (`self.SoftStateMorph`))))
  (set `self.SoftStateAnim` _assoft_state_anim))

(event `Key|R`
  (params (Key :type "Key Structure"))
  (bind _character_collision (`self.Character_Collision`))
  ;[1 1 1] Reset
  (:`Pressed`
    (`SceneComponent.K2_SetWorldLocation` _character_collision (0.0 0.0 1000.0) false false)
    (`PrimitiveComponent.SetPhysicsLinearVelocity` _character_collision (0.0 0.0 0.0) false "None")))

(event `self.ReceiveTick`
  (params (DeltaSeconds :type "Float (single-precision)"))
  (bind _returnvalue (`self.GetInputAxisValue`))
  (bind _returnvalue_2 (`self.GetInputAxisValue`))
  (bind _returnvalue_3 (`SceneComponent.K2_GetComponentLocation` (`self.Character_Collision`)))
  ;[1 1 1] Grounding Detection
  (set `self.FrameTime` (* DeltaSeconds 60.0))
  (bind (_outhit _returnvalue_4) (`KismetSystemLibrary.SphereTraceSingleForObjects` _returnvalue_3 (- _returnvalue_3 (0.0 0.0 30.0)) (`SphereComponent.SphereRadius` (`self.Character_Collision`)) (`|MakeArray` "ObjectTypeQuery1" "ObjectTypeQuery2" :!type "EObjectTypeQuery Enum")))
  (if (and _returnvalue_4 (not (`self.IsGrounded`)))
    (`self.PlayLand`)
    (`self.LandSquish`))
  (set `self.IsGrounded` _returnvalue_4)
  ;[1 1 1] Add Movement Velocity
  (`self.UpdateMovementSounds`)
  (`PrimitiveComponent.AddImpulse` (`self.Character_Collision`) (* (* (`KismetMathLibrary.Normal` (`KismetMathLibrary.MakeVector` _returnvalue_2 _returnvalue (* 0.1 (`KismetMathLibrary.Conv_BoolToDouble` (or (> _returnvalue_2 0.0) (> _returnvalue 0.0)))))) (`self.CurPower`)) (`self.FrameTime`)) "None" false)
  ;[1 1 1] Limit Velocity
  (bind _returnvalue_5 (`PrimitiveComponent.GetPhysicsLinearVelocity` (`self.Character_Collision`) "None"))
  (if (> (`KismetMathLibrary.VSize` _returnvalue_5) (`self.CurVelLim`))
    (`PrimitiveComponent.AddImpulse` (`self.Character_Collision`) (* (* (* (`KismetMathLibrary.Normal` _returnvalue_5) -1) (`self.CurPower`)) (`self.FrameTime`)) "None" false))
  ;[1 1 1] Rotate character models so they are facing the direction of travel and rotate them with morphs so they appear to roll
  (`self.RotateModel`)
  ;[1 1 1] Add Extra Gravity
  (if (`self.AddGravity`)
    (`PrimitiveComponent.AddImpulse` (`self.Character_Collision`) (* (* (0.0 0.0 -1.0) (`self.CurGrav`)) (`self.FrameTime`)) "None" false))
  ;[1 1 1] Countdown Bounce Frame Timer
  (if (<= (`self.BounceTimer`) 0.0)
    (if (`self.BounceTiming`)
      (`PrimitiveComponent.SetPhysMaterialOverride` (`self.Character_Collision`) "/Game/Physics_Materials/SoftHalf_PM.SoftHalf_PM")
      (set `self.BounceTiming` false))
    (else
      (set `self.BounceTimer` (- (`self.BounceTimer`) (`self.FrameTime`)))))
  ;[1 1 1] Countdown Jump Frame Timer
  (if (<= (`self.JumpTimer`) 0.0)
    (set `self.JumpTiming` false)
    (else
      (set `self.JumpTimer` (- (`self.JumpTimer`) (`self.FrameTime`))))))

(event `InputAction|SwitchState`
  (params (Key :type "Key Structure"))
  (bind _mass (`self.Mass`))
  (bind _basegrav (`self.BaseGrav`))
  (bind _basevellim (`self.BaseVelLim`))
  (bind _returnvalue (`KismetStringLibrary.EqualEqual_StrStr` (`self.State`) "float"))
  ;[1 1 1] Switch state
  (:`Pressed`
    (if _returnvalue
      (`PrimitiveComponent.SetEnableGravity` (`self.Character_Collision`) true))
    (`self.TransformModel` (`self.State`) "hard")
    (set `self.State` "hard")
    (set `self.CurPower` (* (`self.BasePower`) (`self.HardMoveMultiplier`) 1.5))
    (set `self.CurVelLim` (* _basevellim (`self.HardMoveMultiplier`)))
    (set `self.CurGrav` (* _basegrav (`self.HardGravMultiplier`)))
    (`PrimitiveComponent.SetMassOverrideInKg` (`self.Character_Collision`) "None" (* _mass (`self.HardMoveMultiplier`)) true)
    (`PrimitiveComponent.SetMaterial` (`self.HardStateMorph`) 0 "/Game/Test_Materials/Hard_TestMat.Hard_TestMat")
    (`PrimitiveComponent.SetPhysMaterialOverride` (`self.Character_Collision`) "/Game/Physics_Materials/Hard_PM.Hard_PM")
    (`SceneComponent.SetRelativeScale3D` (`self.HardStateMorph`) (1.5 1.5 1.5)))
  (:`Released`
    (if (not _returnvalue)
      (`self.TransformModel` (`self.State`) "soft")
      (set `self.State` "soft")
      (set `self.CurPower` (`self.BasePower`))
      (set `self.CurVelLim` _basevellim)
      (set `self.CurGrav` _basegrav)
      (`PrimitiveComponent.SetMassOverrideInKg` (`self.Character_Collision`) "None" _mass true)
      (`PrimitiveComponent.SetPhysMaterialOverride` (`self.Character_Collision`) "/Game/Physics_Materials/SoftFull_PM.SoftFull_PM")
      (set `self.BounceTimer` (`self.BounceTimerSet`))
      (set `self.BounceTiming` true))))

(event `InputAction|Jump`
  (params (Key :type "Key Structure"))
  (bind _character_collision (`self.Character_Collision`))
  ;[1 1 1] Jump while in soft state
  (:`Pressed`
    (if (and (`KismetStringLibrary.EqualEqual_StrStr` (`self.State`) "soft") (`self.IsGrounded`) (not (`self.JumpTiming`)))
      (bind _returnvalue (`PrimitiveComponent.GetPhysicsLinearVelocity` _character_collision "None"))
      (`PrimitiveComponent.SetPhysicsLinearVelocity` _character_collision (`KismetMathLibrary.MakeVector` (.x _returnvalue) (.y _returnvalue)) false "None")
      (`PrimitiveComponent.AddImpulse` _character_collision (0.0 0.0 1000000.0) "None" false)
      (`self.PlayJump`)
      (set `self.JumpTimer` (`self.JumpTimerSet`))
      (set `self.JumpTiming` true))))

(event `self.Character_Collision.OnComponentBeginOverlap`
  (params (OverlappedComponent :type "PrimitiveComponent Object Reference") (OtherActor :type "Actor Object Reference") (OtherComp :type "PrimitiveComponent Object Reference") (OtherBodyIndex :type Integer) (bFromSweep :type Boolean) (SweepResult :type "HitResult Structure (by ref)"))
  (bind _hardstatemorph (`self.HardStateMorph`))
  (bind _character_collision (`self.Character_Collision`))
  ;[1 1 1] Look for powerup overlaps
  (cast `/Game/Blueprints/Float` OtherActor
    (:`then`
      ;[1 1 1] Engage float powerup
      (bind _output_get (set `self.State` "float"))
      (`self.TransformModel` _output_get)
      (`PrimitiveComponent.SetMassOverrideInKg` _character_collision "None" (`self.Mass`) true)
      (`PrimitiveComponent.SetMaterial` _hardstatemorph 0 "/Game/Test_Materials/Helium_TestMat.Helium_TestMat")
      (`PrimitiveComponent.SetPhysMaterialOverride` _character_collision "/Game/Physics_Materials/SoftFull_PM.SoftFull_PM")
      (`PrimitiveComponent.SetEnableGravity` _character_collision false)
      (`SceneComponent.SetRelativeScale3D` _hardstatemorph (2.0 2.0 2.0)))
    (:`CastFailed`
      (cast `/Game/Blueprints/Speed` OtherActor)
      ;[1 1 1] Engage speed powerup
      (set `self.SpeedBoost` true))))

(event `InputAction|SpeedBoost`
  (params (Key :type "Key Structure"))
  (bind _character_collision (`self.Character_Collision`))
  ;[1 1 1] Engage speed powerup
  (:`Pressed`
    (if (`self.SpeedBoost`)
      (bind _returnvalue (`PrimitiveComponent.GetPhysicsLinearVelocity` _character_collision "None"))
      (`PrimitiveComponent.AddImpulse` _character_collision (* (* (`KismetMathLibrary.Normal` _returnvalue) (`self.CurPower`)) (`self.SpeedBoostMultiplier`)) "None" false)
      (set `self.SpeedBoost` false))))

(fn `GetMovementSound`
  (params (State :type String))
  (returns (Sound :type "SoundBase Object Reference"))
  (switch `string` State
    (:`Default`
      (return null))
    (:`soft`
      (return "/Game/Sounds/Blob/soft_movement.soft_movement"))
    (:`hard`
      (return "/Game/Sounds/Blob/hard_movement.hard_movement"))))

(fn `LandSquish`
  (bind _squishmax (`self.SquishMax`))
  (if (`KismetStringLibrary.EqualEqual_StrStr` (`self.State`) "soft")
    (bind _returnvalue (`PrimitiveComponent.GetPhysicsLinearVelocity` (`self.Character_Collision`) "None"))
    (`/Game/Models/Blob/SoftStateAnim.LandSquish` (`self.SoftStateAnim`) (/ (`KismetMathLibrary.FClamp` (`KismetMathLibrary.Abs` (.z _returnvalue)) 0.0 _squishmax) _squishmax))))

(fn `PlayJump`
  (bind _jumplandsound (`self.JumpLandSound`))
  (`AudioComponent.SetSound` _jumplandsound "/Game/Sounds/Blob/hard_jump.hard_jump")
  (`AudioComponent.Play` _jumplandsound 0.0))

(fn `PlayLand`
  (bind _jumplandsound (`self.JumpLandSound`))
  (`AudioComponent.SetSound` _jumplandsound "/Game/Sounds/Blob/soft_land.soft_land")
  (`AudioComponent.Play` _jumplandsound 0.0))

(fn `RotateModel`
  (bind _returnvalue (`PrimitiveComponent.GetPhysicsLinearVelocity` (`self.Character_Collision`) "None"))
  (bind _returnvalue_2 (`KismetMathLibrary.MakeVector` (.x _returnvalue) (.y _returnvalue)))
  (bind _returnvalue_3 (`KismetMathLibrary.VSize` _returnvalue_2))
  (if (> _returnvalue_3 (`self.RotateThreshold`))
    (`SceneComponent.K2_SetRelativeRotation` (`self.HardStateMorph`) (`KismetMathLibrary.Conv_VectorToRotator` _returnvalue_2) false false)
    (`SceneComponent.K2_SetRelativeRotation` (`self.SoftStateMorph`) (`KismetMathLibrary.Conv_VectorToRotator` _returnvalue_2) false false)
    (if (`self.IsGrounded`)
      _
      (else
        _))
    (switch `string` (`self.State`)
      (:`hard`
        (`/Game/Models/Blob/HardStateAnim.Rotate` (`self.HardStateAnim`) _returnvalue_3))
      (:`soft`
        (`/Game/Models/Blob/SoftStateAnim.Rotate` (`self.SoftStateAnim`) _returnvalue_3)))))

(fn `SwitchModel`
  (params (Model :type String))
  (switch `string` Model
    (:`hard`
      (`SceneComponent.SetVisibility` (`self.HardStateMorph`) true false)
      (`SceneComponent.SetVisibility` (`self.SoftStateMorph`) false false))
    (:`soft`
      (`SceneComponent.SetVisibility` (`self.SoftStateMorph`) true false)
      (`SceneComponent.SetVisibility` (`self.HardStateMorph`) false false))))

(fn `TransformModel`
  (params (From :type String) (To :type String))
  (switch `string` From
    (:`hard`
      (switch `string` To
        (:`soft`
          (`/Game/Models/Blob/HardStateAnim.ToSoft` (`self.HardStateAnim`)))))
    (:`soft`
      (switch `string` To
        (:`hard`
          (`/Game/Models/Blob/SoftStateAnim.ToHard` (`self.SoftStateAnim`)))))))

(fn `UpdateMovementSounds`
  (bind _movementsound (`self.MovementSound`))
  ;[1 1 1] Check if character is grounded and not moving
  (if (`self.IsGrounded`)
    (bind _returnvalue (`PrimitiveComponent.GetPhysicsLinearVelocity` (`self.Character_Collision`) "None"))
    (if (== _returnvalue (0.0 0.0 0.0) :`ErrorTolerance` 0.5)
      ;[1 1 1] If not moving reset IsMoving bool and kill sound
      (set `self.IsMoving` false :!label _label)
      (`AudioComponent.Stop` (`self.MovementSound`))
      (else
        ;[1 1 1] If moving check if character is still in the same state as last update
        (if (`KismetStringLibrary.EqualEqual_StrStr` (`self.State`) (`self.SoundState`))
          ;[1 1 1] If in the same state as last update check if the character just started moving
          (if (not (`self.IsMoving`))
            ;[1 1 1] If just started moving or state changed play sound based on state
            (bind _sound (`self.GetMovementSound` (`self.SoundState`) :!label _label_2))
            (`AudioComponent.SetSound` _movementsound _sound)
            (`AudioComponent.Play` _movementsound 0.0)
            (set `self.IsMoving` true))
          (else
            ;[1 1 1] Set sound state to match state
            (set `self.SoundState` (`self.State`))
            (goto _label_2)))))
    (else
      (goto _label))))

(fn `UserConstructionScript`)